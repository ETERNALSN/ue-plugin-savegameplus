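; BP_ExampleSaveActor is an example actor that saves and loads a SaveGamePlus object through overlap events.
; When an overlap begins, it constructs an ExampleSaveGamePlus object, stores a reference to itself in it and saves it to a fixed slot.
; When the overlap ends, it loads that slot with a config specifying the expected header type and class, then prints the success flag and error message.
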(event `self.ReceiveActorBeginOverlap`
  (params (OtherActor :type "Actor Object Reference"))
  (bind _returnvalue (`|GenericCreateObject` "/Script/SaveGamePlus.ExampleSaveGamePlus"))
  (set `ExampleSaveGamePlus.ExampleSaveActor` self _returnvalue)
  (`self.Save` _returnvalue "MySaves/Example"))

(event `self.ReceiveActorEndOverlap`
  (params (OtherActor :type "Actor Object Reference"))
  (bind _outresult (`self.Load` "MySaves/Example" (make `SaveGameLoadConfig` "Example" true false true "/Script/SaveGamePlus.ExampleSaveGamePlus")))
  (bind (_bsuccess _errormessage) (break `SaveGameLoadResult` _outresult))
  (`KismetSystemLibrary.PrintString` (`KismetStringLibrary.Conv_BoolToString` _bsuccess))
  (`KismetSystemLibrary.PrintString` _errormessage))

(fn `UserConstructionScript`)